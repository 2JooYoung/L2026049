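; Player-controllable aircraft pawn that flies forward continuously and fires rockets.
; Tick moves Body along its local X by MoveSpeed scaled by delta time and spins both propellers at a fixed per-frame rate.
; Pitch and Roll axis inputs rotate Body directly, without delta-time scaling.
; Fire spawns BP_Rocket at an offset along world X from Body, without passing its rotation.
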(event `self.ReceiveTick`
  (params (DeltaSeconds :type "Float (single-precision)"))
  (`SceneComponent.K2_AddLocalOffset` (`self.Body`) (`KismetMathLibrary.MakeVector` (* DeltaSeconds (`self.MoveSpeed`))) false false)
  (`SceneComponent.K2_AddLocalRotation` (`self.LeftPropeller`) (`KismetMathLibrary.MakeRotator` 300.0) false false)
  (`SceneComponent.K2_AddLocalRotation` (`self.RightPropeller`) (`KismetMathLibrary.MakeRotator` 300.0) false false))

(event `InputAxis|Pitch`
  (params (AxisValue :type "Float (single-precision)"))
  (`SceneComponent.K2_AddLocalRotation` (`self.Body`) (`KismetMathLibrary.MakeRotator` 0.0 AxisValue) false false))

(event `InputAction|Fire`
  (params (Key :type "Key Structure"))
  (bind (_returnvalue_x _returnvalue_y _returnvalue_z) (`KismetMathLibrary.BreakVector` (`SceneComponent.K2_GetComponentLocation` (`self.Body`))))
  (:`Pressed`
    (`|SpawnActorFromClass` "/Game/Blueprints/BP_Rocket.BP_Rocket_C" (`KismetMathLibrary.MakeTransform` (`KismetMathLibrary.MakeVector` (+ _returnvalue_x 100.0) _returnvalue_y _returnvalue_z)) "Undefined" "MultiplyWithRoot" null null)))

(event `InputAxis|Roll`
  (params (AxisValue :type "Float (single-precision)"))
  (`SceneComponent.K2_AddLocalRotation` (`self.Body`) (`KismetMathLibrary.MakeRotator` AxisValue) false false))

(fn `UserConstructionScript`)